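; BPS_ItemGenerator is a timed item generator that flags when items are ready and reports that state to its ConstructionAsset.
; On BeginPlay, if enabled with no items generated, it waits TimeToGenerate, sets ItemsGenerated and updates the asset's text render.
; ResetTimer clears the flag, restarts the delay and immediately refreshes the text.
; Only the boolean state is handled here, with no item spawning.
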(event Custom|ResetTimer
  (Variables|Default|SetItemsGenerated false)
  (CallFunction|StartTimer)
  (Default|UpdateTextRender (Variables|Core|GetConstructionAsset) (Variables|Default|GetItemsGenerated)))

(event Custom|StartTimer
  (Utilities|FlowControl|Delay (Variables|Default|GetTimeToGenerate))
  (Variables|Default|SetItemsGenerated true)
  (Default|UpdateTextRender (Variables|Core|GetConstructionAsset) (Variables|Default|GetItemsGenerated)))

(event EventBeginPlay
  (if (Variables|Default|GetEnabled)
    (if (not (Variables|Default|GetItemsGenerated))
      (CallFunction|StartTimer))))

(event EventTick
  (params (DeltaSeconds :type Float%20%28single-precision%29)))