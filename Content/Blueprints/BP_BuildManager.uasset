(event EventBeginPlay
  (bind _asbp_player_character (Utilities|Casting|CastToBP_PlayerCharacter (Game|GetPlayerCharacter 0)))
  (Variables|Core|SetPlayerCharacter _asbp_player_character)
  (Variables|/Game/Blueprints/Core/BP_PlayerCharacter.BP_PlayerCharacter_C|SetBuildManager (Variables|Core|GetPlayerCharacter) self)
  (bind _asbp_player_controller (Utilities|Casting|CastToBP_PlayerController (Game|GetPlayerController 0)))
  (Variables|Core|SetPlayerController _asbp_player_controller)
  (Variables|/Game/Blueprints/Core/BP_PlayerController.BP_PlayerController_C|SetBuildManager (Variables|Core|GetPlayerController) self)
  (Variables|Core|SetMainHUD (Variables|/Game/Blueprints/Core/BP_PlayerController.BP_PlayerController_C|GetMainHUD (Variables|Core|GetPlayerController)))
  (Variables|/Game/Blueprints/Core/BP_MainHUD.BP_MainHUD_C|SetBuildManager (Variables|Core|GetMainHUD) self)
  (CallFunction|GetResourcesData)
  (Default|LoadSceneObjects (Variables|Core|GetPlayerController)))

(event EventActorBeginOverlap
  (params (OtherActor :type Actor%20Object%20Reference)))

(event EventTick
  (params (DeltaSeconds :type Float%20%28single-precision%29)))

(fn ConstructionScript)

(fn LoadObjects
  (for _array_element (Variables|Default|GetSceneObjects)
    (Game|SpawnActorfromClass (.Asset (Utilities|Struct|BreakS_SceneObject _array_element)) (.WorldPosition (Utilities|Struct|BreakS_SceneObject _array_element)) "Undefined" 0 0)))

(fn GetResourcesData
  (Utilities|FlowControl|Sequence
    (:then_0
      (Variables|Resources|SetMass (Utilities|Struct|BreakS_ConstructionResources (Variables|/Game/Blueprints/Core/BP_PlayerController.BP_PlayerController_C|GetResources (Variables|Core|GetPlayerController)))))))

(fn CreateTempObject
  (params (ObjectName :type Name))
  (Variables|Default|SetBuildMode true)
  (bind _returnvalue (Game|SpawnActorfromClass "/Game/Blueprints/BP_ConstructionDummy.BP_ConstructionDummy_C" (LocalVariables|GetNullTransform) "Undefined" 0 0))
  (Variables|Construction|SetConstructionDummy _returnvalue)
  (Default|GetAssetInfo _returnvalue ObjectName)
  (Class|Actor|AttachRootComponentto _returnvalue (Variables|/Game/Blueprints/Core/BP_PlayerCharacter.BP_PlayerCharacter_C|GetConstructionRoot (Variables|/Game/Blueprints/Core/BP_PlayerController.BP_PlayerController_C|GetPlayerCharacter (Variables|Core|GetPlayerController))) "None" "KeepRelativeOffset" true)
  (Variables|/Game/Blueprints/BP_ConstructionDummy.BP_ConstructionDummy_C|SetInBuildMode (Variables|Construction|GetConstructionDummy) true))

(fn AddSceneObject
  (params (NewObject :type BP%20Construction%20Asset%20Class%20Reference) (ActorTransform :type Transform))
  (Utilities|Array|Add (Variables|Default|GetSceneObjects) (Utilities|Struct|MakeS_SceneObject NewObject ActorTransform))
  (Default|SaveGameData (Variables|Core|GetPlayerController))
  (Variables|Default|SetBuildMode false))