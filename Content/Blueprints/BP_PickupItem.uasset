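; BP_PickupItem is a pickup actor that the player collects by pressing the Action input while inside its trigger volume.
; Overlapping the volume enables input on the actor and shows a text prompt, and leaving reverses both, with no check on the overlapping actor.
; Instant items pass Value to the cached BP_PlayerCharacter's health, stamina or resource function by ItemType; others add ItemName to inventory, then the pickup destroys itself.
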(event OnComponentBeginOverlap(TriggerVolume)
  (params (OtherActor :type Actor%20Object%20Reference) (OtherComp :type Primitive%20Component%20Object%20Reference) (OtherBodyIndex :type Integer) (bFromSweep :type Boolean) (SweepResult :type Hit%20Result%20Structure%20%28by%20ref%29))
  (Input|EnableInput (Game|GetPlayerController 0))
  (Rendering|SetVisibility (Variables|Default|GetTextRender) true false))

(event OnComponentEndOverlap(TriggerVolume)
  (params (OtherActor :type Actor%20Object%20Reference) (OtherComp :type Primitive%20Component%20Object%20Reference) (OtherBodyIndex :type Integer))
  (Input|DisableInput (Game|GetPlayerController 0))
  (Rendering|SetVisibility (Variables|Default|GetTextRender) false false))

(event EventBeginPlay
  (bind _asbp_player_character (Utilities|Casting|CastToBP_PlayerCharacter (Game|GetPlayerCharacter 0)))
  (Variables|Core|SetPlayerCharacter _asbp_player_character))

(event EventActorBeginOverlap
  (params (OtherActor :type Actor%20Object%20Reference)))

(event EventTick
  (params (DeltaSeconds :type Float%20%28single-precision%29)))

(event Input|ActionEvents|InputActionAction
  (params (Key :type Key%20Structure :default "AnyKey"))
  (bind _value (Variables|Default|GetValue))
  (bind _playercharacter (Variables|Core|GetPlayerCharacter))
  (:Pressed
    (if (Variables|Default|GetInstantEffect)
      (switch Utilities|FlowControl|Switch|SwitchonE_ItemType (Variables|Default|GetItemType)
        (:NewEnumerator0
          (Default|DamageHealth _playercharacter _value))
        (:NewEnumerator1
          (Default|DamageStamina _playercharacter _value))
        (:NewEnumerator2
          (Default|AddResource (Variables|Core|GetPlayerCharacter) (Math|Float|Truncate (Variables|Default|GetValue)))))
      (else
        (Default|AddItemtoInventory (Variables|Core|GetPlayerCharacter) (Variables|Default|GetItemName))))
    (Actor|DestroyActor)))

(fn ConstructionScript)