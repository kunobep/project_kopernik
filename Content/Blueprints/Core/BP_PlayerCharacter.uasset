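; BP_PlayerCharacter is the player pawn, handling movement, look, camera view, survival stats and item pickup.
; Movement follows control yaw only, and ViewChange toggles the camera between first- and third-person roots.
; Each Tick drains stamina, faster while moving, then damages health once it runs out, without delta-time scaling.
; Helper functions damage stats, add mass to BuildManager, and append data-table items to the inventory, refreshing its widget.
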(event EventBeginPlay
  (bind _asbp_player_controller (Utilities|Casting|CastToBP_PlayerController (Game|GetPlayerController 0)))
  (Variables|Core|SetPlayerController _asbp_player_controller))

(event EventActorBeginOverlap
  (params (OtherActor :type Actor%20Object%20Reference)))

(event EventTick
  (params (DeltaSeconds :type Float%20%28single-precision%29))
  (CallFunction|CalculateStaminaConsumption))

(event Input|ActionEvents|InputActionViewChange
  (params (Key :type Key%20Structure :default "AnyKey"))
  ;[1 1 1] Controls
  (:Pressed
    (CallFunction|ChangeCameraView)))

(event Input|AxisEvents|InputAxisLookUp
  (params (AxisValue :type Float%20%28single-precision%29))
  ;[1 1 1] Controls
  (Pawn|Input|AddControllerPitchInput AxisValue))

(event Input|AxisEvents|InputAxisTurn
  (params (AxisValue :type Float%20%28single-precision%29))
  ;[1 1 1] Controls
  (Pawn|Input|AddControllerYawInput AxisValue))

(event Input|AxisEvents|InputAxisMoveRight
  (params (AxisValue :type Float%20%28single-precision%29))
  ;[1 1 1] Controls
  (Pawn|Input|AddMovementInput (Math|Vector|GetRightVector (Math|Rotator|MakeRotator 0.0 0.0 (.Yaw (Math|Rotator|BreakRotator (Pawn|GetControlRotation :!class /Script/Engine.Pawn))))) AxisValue false))

(event Input|AxisEvents|InputAxisMoveForward
  (params (AxisValue :type Float%20%28single-precision%29))
  ;[1 1 1] Controls
  (Pawn|Input|AddMovementInput (Math|Vector|GetForwardVector (Math|Rotator|MakeRotator 0.0 0.0 (.Yaw (Math|Rotator|BreakRotator (Pawn|GetControlRotation :!class /Script/Engine.Pawn))))) AxisValue false))

(fn ConstructionScript)

(fn CalculateStaminaConsumption
  (if (> (Variables|PlayerData|GetPlayerStamina) 0.0)
    (LocalVariables|SetCurrentStaminaConsumption (Variables|Defaults|GetDefaultStaminaConsumption))
    (if (Math|Vector|NotEqual(Vector) (Transformation|GetVelocity) "0, 0, 0" 0.0001)
      (LocalVariables|SetCurrentStaminaConsumption (+ (LocalVariables|GetCurrentStaminaConsumption) (Variables|Defaults|GetMovingStaminaConsumption))))
    (Variables|PlayerData|SetPlayerStamina (- (Variables|PlayerData|GetPlayerStamina) (* (LocalVariables|GetCurrentStaminaConsumption) 0.01)))
    (else
      (CallFunction|DamageHealth (Variables|Defaults|GetHealthDamageWithoutStamina)))))

(fn DamageHealth
  (params (Damage :type Float%20%28single-precision%29))
  (Variables|PlayerData|SetPlayerHealth (- (Variables|PlayerData|GetPlayerHealth) Damage)))

(fn ChangeCameraView
  (bind _output_get (Variables|Default|SetCameraState (not (Variables|Default|GetCameraState))))
  (if _output_get
    (Class|SceneComponent|Attachto (Variables|Default|GetCamera) (Variables|Default|GetCameraRoot3P) "None" "KeepRelativeOffset" true)
    (else
      (Class|SceneComponent|Attachto (Variables|Default|GetCamera) (Variables|Default|GetCameraRoot1P) "None" "KeepRelativeOffset" true))))

(fn DamageStamina
  (params (Damage :type Float%20%28single-precision%29))
  (Variables|PlayerData|SetPlayerStamina (- (Variables|PlayerData|GetPlayerStamina) Damage)))

(fn AddResource
  (params (Value :type Integer))
  (bind _buildmanager (Variables|Core|GetBuildManager))
  (Variables|/Game/Blueprints/BP_BuildManager.BP_BuildManager_C|SetMass _buildmanager (+ Value (Variables|/Game/Blueprints/BP_BuildManager.BP_BuildManager_C|GetMass _buildmanager))))

(fn AddItemtoInventory
  (params (ItemName :type Name))
  (bind _mainhud (Variables|Core|GetMainHUD))
  (bind _inventorymenuwidget (Variables|/Game/Blueprints/Core/BP_MainHUD.BP_MainHUD_C|GetInventoryMenuWidget _mainhud))
  (bind _returnvalue (Utilities|GetDataTableRow "/Game/Blueprints/DataTables/DB_InventoryItems.DB_InventoryItems" ItemName)
    (:then
      (Utilities|Array|Add (Variables|PlayerData|GetPlayerItems) _returnvalue)
      (Utilities|IsValid _inventorymenuwidget
        (:Is%20Valid
          (Default|UpdateInventory _inventorymenuwidget))))))