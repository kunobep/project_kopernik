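; Main HUD that owns the player's UI: a persistent stats widget plus on-demand construction, inventory and crafting menus.
; On BeginPlay it caches the controller, character and the controller's BuildManager, creates the stats widget and registers itself with controller and character.
; Tick pushes health, stamina and mass into the stats widget.
; Load functions create and wire each menu as CurrentWidget, flagging ActiveWidget; CloseCurrentWidget removes it.
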(event EventBeginPlay
  (bind _asbp_player_controller (Utilities|Casting|CastToBP_PlayerController (Game|GetPlayerController 0)))
  (bind _output_get (Variables|Core|SetPlayerController _asbp_player_controller))
  (bind _buildmanager (Default|PushCore _output_get))
  (bind _asbp_player_character (Utilities|Casting|CastToBP_PlayerCharacter (Game|GetPlayerCharacter 0)))
  (Variables|Core|SetPlayerCharacter _asbp_player_character)
  (Variables|Core|SetBuildManager _buildmanager)
  (CallFunction|LoadMainWidgets)
  (Variables|/Game/Blueprints/Core/BP_PlayerController.BP_PlayerController_C|SetMainHUD (Variables|Core|GetPlayerController) self)
  (Variables|/Game/Blueprints/Core/BP_PlayerCharacter.BP_PlayerCharacter_C|SetMainHUD (Variables|Core|GetPlayerCharacter) self))

(event EventActorBeginOverlap
  (params (OtherActor :type Actor%20Object%20Reference)))

(event EventTick
  (params (DeltaSeconds :type Float%20%28single-precision%29))
  (bind _playercharacter (Variables|Core|GetPlayerCharacter))
  (Utilities|FlowControl|Sequence
    (:then_0
      (Default|UpdateData (Variables|Widgets|GetPlayerStatsWidget) (Variables|/Game/Blueprints/Core/BP_PlayerCharacter.BP_PlayerCharacter_C|GetPlayerHealth _playercharacter) (Variables|/Game/Blueprints/Core/BP_PlayerCharacter.BP_PlayerCharacter_C|GetPlayerStamina _playercharacter) (Variables|/Game/Blueprints/BP_BuildManager.BP_BuildManager_C|GetMass (Variables|Core|GetBuildManager))))))

(fn ConstructionScript)

(fn LoadMainWidgets
  (Utilities|FlowControl|Sequence
    (:then_0
      (bind _returnvalue (UserInterface|CreateWidget "/Game/Blueprints/UI/UI_PlayerStats.UI_PlayerStats_C" (Variables|Core|GetPlayerController)))
      (Variables|Widgets|SetPlayerStatsWidget _returnvalue)
      (UserInterface|Viewport|AddtoViewport (Variables|Widgets|GetPlayerStatsWidget) 0))))

(fn LoadBuildMenu
  (params (PlayerCharacter :type BP%20Player%20Character%20Object%20Reference) (BuildManager :type BP%20Build%20Manager%20Object%20Reference))
  (Variables|Default|SetActiveWidget true)
  (bind _returnvalue (UserInterface|CreateWidget "/Game/Blueprints/UI/UI_ConstructionMenu.UI_ConstructionMenu_C" (Variables|Core|GetPlayerController)))
  (Variables|Widgets|SetBuildMenuWidget _returnvalue)
  (Utilities|FlowControl|Sequence
    (:then_0
      (UserInterface|Viewport|AddtoViewport (Variables|Widgets|GetBuildMenuWidget) 0))
    (:then_1
      (Variables|/Game/Blueprints/UI/UI_ConstructionMenu.UI_ConstructionMenu_C|SetPlayerCharacter (Variables|Widgets|GetBuildMenuWidget) PlayerCharacter))
    (:then_2
      (Variables|/Game/Blueprints/UI/UI_ConstructionMenu.UI_ConstructionMenu_C|SetBuildManager (Variables|Widgets|GetBuildMenuWidget) BuildManager))
    (:then_3
      (Variables|Widgets|SetCurrentWidget (Variables|Widgets|GetBuildMenuWidget)))
    (:then_4
      (Variables|/Game/Blueprints/UI/UI_ConstructionMenu.UI_ConstructionMenu_C|SetMainHUD (Variables|Widgets|GetBuildMenuWidget) self))))

(fn LoadInventoryMenu
  (params (BuildManager :type BP%20Build%20Manager%20Object%20Reference) (PlayerController :type BP%20Player%20Controller%20Object%20Reference))
  (Variables|Default|SetActiveWidget true)
  (bind _returnvalue (UserInterface|CreateWidget "/Game/Blueprints/UI/UI_PlayerInventory.UI_PlayerInventory_C" (Variables|Core|GetPlayerController)))
  (Variables|Widgets|SetInventoryMenuWidget _returnvalue)
  (Utilities|FlowControl|Sequence
    (:then_0
      (UserInterface|Viewport|AddtoViewport (Variables|Widgets|GetInventoryMenuWidget) 0))
    (:then_1
      (Variables|/Game/Blueprints/UI/UI_PlayerInventory.UI_PlayerInventory_C|SetBuildManager (Variables|Widgets|GetInventoryMenuWidget) BuildManager))
    (:then_2
      (Variables|Widgets|SetCurrentWidget (Variables|Widgets|GetInventoryMenuWidget)))
    (:then_3
      (Variables|/Game/Blueprints/UI/UI_PlayerInventory.UI_PlayerInventory_C|SetPlayerController (Variables|Widgets|GetInventoryMenuWidget) PlayerController))
    (:then_4
      (Variables|/Game/Blueprints/UI/UI_PlayerInventory.UI_PlayerInventory_C|SetMainHUD (Variables|Widgets|GetInventoryMenuWidget) self))))

(fn CloseCurrentWidget
  (Variables|Default|SetActiveWidget false)
  (Utilities|IsValid (Variables|Widgets|GetCurrentWidget)
    (:Is%20Valid
      (Widget|RemovefromParent (Variables|Widgets|GetCurrentWidget)))))

(fn LoadCraftMenu
  (params (PlayerController :type BP%20Player%20Controller%20Object%20Reference))
  (Variables|Default|SetActiveWidget true)
  (bind _returnvalue (UserInterface|CreateWidget "/Game/Blueprints/UI/UI_CraftMenu.UI_CraftMenu_C" PlayerController))
  (Variables|Widgets|SetCraftMenuWidget _returnvalue)
  (Utilities|FlowControl|Sequence
    (:then_0
      (UserInterface|Viewport|AddtoViewport (Variables|Widgets|GetCraftMenuWidget) 0))
    (:then_1
      (Variables|/Game/Blueprints/UI/UI_CraftMenu.UI_CraftMenu_C|SetMainHUD (Variables|Widgets|GetCraftMenuWidget) self))
    (:then_2
      (Variables|/Game/Blueprints/UI/UI_CraftMenu.UI_CraftMenu_C|SetPlayerCharacter (Variables|Widgets|GetCraftMenuWidget) (Variables|Core|GetPlayerCharacter)))
    (:then_3
      (Variables|Widgets|SetCurrentWidget (Variables|Widgets|GetCraftMenuWidget)))))