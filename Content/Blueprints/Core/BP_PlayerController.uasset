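; Player controller that owns save/load and routes menu input for a survival-style building game.
; On BeginPlay it loads the save slot, applies health, stamina and items to the character, then starts a Delay-based self-recalling autosave.
; Saving gathers character and BuildManager state; LoadSceneObjects returns saved objects to BuildManager and reads construction items from a DataTable.
; Input toggles build, inventory and craft widgets through MainHUD, or cancels build placement.
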(event Custom|Autosave
  (Utilities|FlowControl|Delay (Variables|Default|GetAutosaveInterval))
  (if (Variables|Default|GetAutosaveEnabled)
    (CallFunction|SaveGameData)
    (CallFunction|Autosave)))

(event EventBeginPlay
  (bind _asbp_player_character (Utilities|Casting|CastToBP_PlayerCharacter (Game|GetPlayerCharacter 0)))
  (Variables|Core|SetPlayerCharacter _asbp_player_character)
  (CallFunction|LoadGameData)
  (CallFunction|SetPlayerData)
  (CallFunction|Autosave))

(event EventTick
  (params (DeltaSeconds :type Float%20%28single-precision%29)))

(event Input|ActionEvents|InputActionCloseActionMenu
  (params (Key :type Key%20Structure :default "AnyKey"))
  (:Pressed
    (bind _inventorymenuwidget (Variables|/Game/Blueprints/Core/BP_MainHUD.BP_MainHUD_C|GetInventoryMenuWidget (Variables|Core|GetMainHUD))
      (:then
        (bind _actionmenu (Variables|/Game/Blueprints/UI/UI_PlayerInventory.UI_PlayerInventory_C|GetActionMenu _inventorymenuwidget)
          (:then
            (Widget|RemovefromParent _actionmenu))
          (:else)))
      (:else))))

(event Input|ActionEvents|InputActionExit
  (params (Key :type Key%20Structure :default "AnyKey"))
  (:Pressed
    (if (Variables|/Game/Blueprints/BP_BuildManager.BP_BuildManager_C|GetBuildMode (Variables|Core|GetBuildManager))
      (Actor|DestroyActor (Variables|/Game/Blueprints/BP_BuildManager.BP_BuildManager_C|GetConstructionDummy (Variables|Core|GetBuildManager)))
      (Variables|/Game/Blueprints/BP_BuildManager.BP_BuildManager_C|SetBuildMode (Variables|Core|GetBuildManager) false))))

(event Input|ActionEvents|InputActionQ
  (params (Key :type Key%20Structure :default "AnyKey"))
  (:Pressed
    (if (Variables|/Game/Blueprints/BP_BuildManager.BP_BuildManager_C|GetBuildMode (Variables|Core|GetBuildManager))
      (Actor|DestroyActor (Variables|/Game/Blueprints/BP_BuildManager.BP_BuildManager_C|GetConstructionDummy (Variables|Core|GetBuildManager)))
      (Variables|/Game/Blueprints/BP_BuildManager.BP_BuildManager_C|SetBuildMode (Variables|Core|GetBuildManager) false))))

(event Input|ActionEvents|InputActionCraftMenu
  (params (Key :type Key%20Structure :default "AnyKey"))
  (:Pressed
    (if (Variables|/Game/Blueprints/Core/BP_MainHUD.BP_MainHUD_C|GetActiveWidget (Variables|Core|GetMainHUD))
      (Variables|/Game/Blueprints/Core/BP_MainHUD.BP_MainHUD_C|GetCraftMenuWidget (Variables|Core|GetMainHUD)
        (:then
          (Default|CloseCurrentWidget (Variables|Core|GetMainHUD)))
        (:else))
      (else
        (Default|LoadCraftMenu (Variables|Core|GetMainHUD) self)))))

(event Input|ActionEvents|InputActionInventory
  (params (Key :type Key%20Structure :default "AnyKey"))
  (:Pressed
    (if (Variables|/Game/Blueprints/Core/BP_MainHUD.BP_MainHUD_C|GetActiveWidget (Variables|Core|GetMainHUD))
      (Utilities|IsValid (Variables|/Game/Blueprints/Core/BP_MainHUD.BP_MainHUD_C|GetInventoryMenuWidget (Variables|Core|GetMainHUD))
        (:Is%20Valid
          (Default|CloseCurrentWidget (Variables|Core|GetMainHUD))))
      (else
        (Default|LoadInventoryMenu (Variables|Core|GetMainHUD) (Variables|Core|GetBuildManager) self)))))

(event Input|ActionEvents|InputActionCloseMenu
  (params (Key :type Key%20Structure :default "AnyKey"))
  (:Pressed
    (Default|CloseCurrentWidget (Variables|Core|GetMainHUD))))

(event Input|ActionEvents|InputActionBuildMenu
  (params (Key :type Key%20Structure :default "AnyKey"))
  (:Pressed
    (if (Variables|/Game/Blueprints/Core/BP_MainHUD.BP_MainHUD_C|GetActiveWidget (Variables|Core|GetMainHUD))
      (Utilities|IsValid (Variables|/Game/Blueprints/Core/BP_MainHUD.BP_MainHUD_C|GetBuildMenuWidget (Variables|Core|GetMainHUD))
        (:Is%20Valid
          (Default|CloseCurrentWidget (Variables|Core|GetMainHUD))))
      (else
        (Default|LoadBuildMenu (Variables|Core|GetMainHUD) (Variables|Core|GetPlayerCharacter) (Variables|Core|GetBuildManager))
        (Variables|/Game/Blueprints/Core/BP_PlayerCharacter.BP_PlayerCharacter_C|SetCameraState (Variables|Core|GetPlayerCharacter) true)
        (Default|ChangeCameraView (Variables|Core|GetPlayerCharacter))))))

(fn ConstructionScript)

(fn SetPlayerData
  (bind _playercharacter (Variables|Core|GetPlayerCharacter))
  (bind _playerdata (Variables|SaveData|GetPlayerData))
  (bind (_playerhealth _playerstamina) (Utilities|Struct|BreakS_PlayerData _playerdata))
  (Utilities|FlowControl|Sequence
    (:then_0
      (Variables|/Game/Blueprints/Core/BP_PlayerCharacter.BP_PlayerCharacter_C|SetPlayerHealth _playercharacter _playerhealth))
    (:then_1
      (Variables|/Game/Blueprints/Core/BP_PlayerCharacter.BP_PlayerCharacter_C|SetPlayerStamina _playercharacter _playerstamina))
    (:then_2
      (Variables|/Game/Blueprints/Core/BP_PlayerCharacter.BP_PlayerCharacter_C|SetPlayerItems _playercharacter (Variables|SaveData|GetPlayerItems)))))

(fn SaveGameData
  (CallFunction|GetSaveData)
  (bind _returnvalue (SaveGame|CreateSaveGameObject "/Game/Blueprints/Core/BP_SaveGame.BP_SaveGame_C"))
  (bind _asbp_save_game (Utilities|Casting|CastToBP_SaveGame _returnvalue))
  (Variables|Core|SetSaveGame _asbp_save_game)
  (Variables|/Game/Blueprints/Core/BP_SaveGame.BP_SaveGame_C|SetPlayerData (Variables|Core|GetSaveGame) (Variables|SaveData|GetPlayerData))
  (Variables|/Game/Blueprints/Core/BP_SaveGame.BP_SaveGame_C|SetSceneObjects (Variables|Core|GetSaveGame) (Variables|SaveData|GetSceneObjects))
  (Variables|/Game/Blueprints/Core/BP_SaveGame.BP_SaveGame_C|SetResources (Variables|Core|GetSaveGame) (Variables|SaveData|GetResources))
  (Variables|/Game/Blueprints/Core/BP_SaveGame.BP_SaveGame_C|SetPlayerItems (Variables|Core|GetSaveGame) (Variables|SaveData|GetPlayerItems))
  (Variables|/Game/Blueprints/Core/BP_SaveGame.BP_SaveGame_C|SetCraftObjects (Variables|Core|GetSaveGame) (Variables|Default|GetCraftObjects))
  (SaveGame|SaveGametoSlot (Variables|Core|GetSaveGame) "SaveSlot"))

(fn LoadGameData
  (SaveGame|CreateSaveGameObject "/Game/Blueprints/Core/BP_SaveGame.BP_SaveGame_C")
  (bind _returnvalue (SaveGame|LoadGamefromSlot "SaveSlot"))
  (bind _asbp_save_game (Utilities|Casting|CastToBP_SaveGame _returnvalue))
  (Variables|Core|SetSaveGame _asbp_save_game)
  (Variables|SaveData|SetPlayerData (Variables|/Game/Blueprints/Core/BP_SaveGame.BP_SaveGame_C|GetPlayerData (Variables|Core|GetSaveGame)))
  (Variables|SaveData|SetSceneObjects (Variables|/Game/Blueprints/Core/BP_SaveGame.BP_SaveGame_C|GetSceneObjects (Variables|Core|GetSaveGame)))
  (Variables|SaveData|SetResources (Variables|/Game/Blueprints/Core/BP_SaveGame.BP_SaveGame_C|GetResources (Variables|Core|GetSaveGame)))
  (Variables|SaveData|SetPlayerItems (Variables|/Game/Blueprints/Core/BP_SaveGame.BP_SaveGame_C|GetPlayerItems (Variables|Core|GetSaveGame)))
  (Variables|Default|SetCraftObjects (Variables|/Game/Blueprints/Core/BP_SaveGame.BP_SaveGame_C|GetCraftObjects (Variables|Core|GetSaveGame))))

(fn LoadSceneObjects
  (Utilities|FlowControl|Sequence
    (:then_0
      (Variables|/Game/Blueprints/BP_BuildManager.BP_BuildManager_C|SetSceneObjects (Variables|Core|GetBuildManager) (Variables|SaveData|GetSceneObjects))
      (Variables|/Game/Blueprints/BP_BuildManager.BP_BuildManager_C|SetCraftObjects (Variables|Core|GetBuildManager) (Variables|Default|GetCraftObjects))
      (Default|LoadObjects (Variables|Core|GetBuildManager)))
    (:then_1
      (bind _outrownames (DataTable|GetDataTableRowNames "/Game/Blueprints/DataTables/DB_ConstructionItems.DB_ConstructionItems"))
      (for _array_element _outrownames
        (bind _returnvalue (Utilities|GetDataTableRow "/Game/Blueprints/DataTables/DB_ConstructionItems.DB_ConstructionItems" _array_element)
          (:then
            (Utilities|Array|Add (Variables|Default|GetConstructionItems) _returnvalue)))))))

(fn GetSaveData
  (bind _buildmanager (Variables|Core|GetBuildManager))
  (bind _playercharacter (Variables|Core|GetPlayerCharacter))
  (Utilities|FlowControl|Sequence
    (:then_0
      (Variables|SaveData|SetResources (Utilities|Struct|MakeS_ConstructionResources (Variables|/Game/Blueprints/BP_BuildManager.BP_BuildManager_C|GetMass _buildmanager))))
    (:then_1
      (Variables|SaveData|SetSceneObjects (Variables|/Game/Blueprints/BP_BuildManager.BP_BuildManager_C|GetSceneObjects _buildmanager)))
    (:then_2
      (Variables|SaveData|SetPlayerData (Utilities|Struct|MakeS_PlayerData (Variables|/Game/Blueprints/Core/BP_PlayerCharacter.BP_PlayerCharacter_C|GetPlayerHealth _playercharacter) (Variables|/Game/Blueprints/Core/BP_PlayerCharacter.BP_PlayerCharacter_C|GetPlayerStamina _playercharacter))))
    (:then_3
      (Variables|SaveData|SetPlayerItems (Variables|/Game/Blueprints/Core/BP_PlayerCharacter.BP_PlayerCharacter_C|GetPlayerItems _playercharacter)))
    (:then_4
      (Variables|Default|SetCraftObjects (Variables|/Game/Blueprints/BP_BuildManager.BP_BuildManager_C|GetCraftObjects _buildmanager)))))

(fn PushCore
  (return (Variables|Core|GetPlayerCharacter) (Variables|Core|GetBuildManager) (Variables|Core|GetMainHUD)))

(fn SetBuildManager
  (params (BuildManager :type BP%20Build%20Manager%20Object%20Reference))
  (Variables|Core|SetBuildManager BuildManager))