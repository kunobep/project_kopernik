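; BP_ConstructionDummy is the placement preview actor for building, showing a construction item's mesh looked up by name in DB_ConstructionItems.
; While in build mode it takes input, spinning on yaw while RotateObject is held.
; The Action input spawns the real item at its transform, registers it with the player controller's BuildManager, charges stamina and Mass, loads its sockets, then destroys the dummy.
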(event EventBeginPlay
  (bind _asbp_player_controller (Utilities|Casting|CastToBP_PlayerController (Game|GetPlayerController 0)))
  (bind _output_get (Variables|Core|SetPlayerController _asbp_player_controller))
  (bind _buildmanager (Default|PushCore _output_get))
  (Variables|Core|SetBuildManager _buildmanager)
  (bind _asbp_player_character (Utilities|Casting|CastToBP_PlayerCharacter (Game|GetPlayerCharacter 0)))
  (Variables|Core|SetPlayerCharacter _asbp_player_character))

(event EventActorBeginOverlap
  (params (OtherActor :type Actor%20Object%20Reference)))

(event EventTick
  (params (DeltaSeconds :type Float%20%28single-precision%29))
  (bind _returnvalue (Transformation|GetActorRotation))
  (bind _playercontroller (Variables|Core|GetPlayerController))
  (bind _yaw (Math|Rotator|BreakRotator _returnvalue))
  (if (Variables|Default|GetInBuildMode)
    (Input|EnableInput _playercontroller)
    (if (Variables|Default|GetRotateObject)
      (Variables|Default|SetYawPos (+ _yaw (Variables|Default|GetRotateSpeed)))
      (else
        (Variables|Default|SetYawPos _yaw)))
    (Transformation|SetActorRotation (Math|Rotator|MakeRotator 0.0 0.0 (Variables|Default|GetYawPos)))
    (else
      (Input|DisableInput _playercontroller))))

(event Input|ActionEvents|InputActionRotateObject
  (params (Key :type Key%20Structure :default "AnyKey"))
  (:Pressed
    (Variables|Default|SetRotateObject true))
  (:Released
    (Variables|Default|SetRotateObject false)))

(event Input|ActionEvents|InputActionAction
  (params (Key :type Key%20Structure :default "AnyKey"))
  (:Pressed
    (CallFunction|PlaceObject)
    (Actor|DestroyActor)))

(fn ConstructionScript)

(fn PlaceObject
  (bind _defaultsceneroot (Variables|Default|GetDefaultSceneRoot))
  (bind _returnvalue (Transformation|GetWorldTransform _defaultsceneroot))
  (bind _returnvalue_2 (Utilities|GetDataTableRow "/Game/Blueprints/DataTables/DB_ConstructionItems.DB_ConstructionItems" (Variables|AssetData|GetAssetName))
    (:then
      (bind _returnvalue_3 (Game|SpawnActorfromClass (.ItemActor (Utilities|Struct|BreakS_ConstructionItem _returnvalue_2)) _returnvalue "Undefined" 0 0))
      (Default|AddSceneObject (Variables|Core|GetBuildManager) (.ItemActor (Utilities|Struct|BreakS_ConstructionItem _returnvalue_2)) _returnvalue)
      (Utilities|FlowControl|Sequence
        (:then_0
          (Default|DamageStamina (Variables|Core|GetPlayerCharacter) (Variables|AssetData|GetAssetStaminaCost)))
        (:then_1
          (Default|AddResource (Variables|Core|GetPlayerCharacter) (* (Utilities|Struct|BreakS_ConstructionResources (Variables|AssetData|GetAssetResourceCost)) -1)))
        (:then_2
          (Default|LoadSockets _returnvalue_3))
        (:then_3
          (Variables|/Game/Blueprints/BP_ConstructionAsset.BP_ConstructionAsset_C|SetBuildManager _returnvalue_3 (Variables|Core|GetBuildManager)))))))

(fn GetAssetInfo
  (params (AssetName :type Name))
  (Variables|AssetData|SetAssetName AssetName)
  (bind _returnvalue (Utilities|GetDataTableRow "/Game/Blueprints/DataTables/DB_ConstructionItems.DB_ConstructionItems" (Variables|AssetData|GetAssetName))
    (:then
      (Utilities|FlowControl|Sequence
        (:then_0
          (Components|StaticMesh|SetStaticMesh (Variables|Default|GetMesh) (.ItemMesh (Utilities|Struct|BreakS_ConstructionItem _returnvalue))))
        (:then_1
          (Variables|AssetData|SetAssetActor (.ItemActor (Utilities|Struct|BreakS_ConstructionItem _returnvalue))))
        (:then_2
          (Variables|AssetData|SetAssetStaminaCost (.ItemStaminaCost (Utilities|Struct|BreakS_ConstructionItem _returnvalue))))
        (:then_3
          (Variables|AssetData|SetAssetResourceCost (.ItemResourceCost (Utilities|Struct|BreakS_ConstructionItem _returnvalue))))))))