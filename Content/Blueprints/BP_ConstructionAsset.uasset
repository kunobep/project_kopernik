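; Base actor for a construction asset that generates items the player can collect into their inventory.
; A trigger volume enables and disables the actor's input as overlaps begin and end, so the Action press works nearby.
; When the item generator component is enabled and has items ready, the press adds them to the player character and resets its timer.
; The generator receives a self reference, and a helper function toggles the text render's visibility.
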(event OnComponentBeginOverlap(TriggerVolume)
  (params (OtherActor :type Actor%20Object%20Reference) (OtherComp :type Primitive%20Component%20Object%20Reference) (OtherBodyIndex :type Integer) (bFromSweep :type Boolean) (SweepResult :type Hit%20Result%20Structure%20%28by%20ref%29))
  (Input|EnableInput (Game|GetPlayerController 0)))

(event OnComponentEndOverlap(TriggerVolume)
  (params (OtherActor :type Actor%20Object%20Reference) (OtherComp :type Primitive%20Component%20Object%20Reference) (OtherBodyIndex :type Integer))
  (Input|DisableInput (Game|GetPlayerController 0)))

(event EventBeginPlay
  (bind _asbp_player_controller (Utilities|Casting|CastToBP_PlayerController (Game|GetPlayerController 0)))
  (Variables|Default|SetPlayerController _asbp_player_controller)
  (bind _asbp_player_character (Utilities|Casting|CastToBP_PlayerCharacter (Game|GetPlayerCharacter 0)))
  (Variables|Default|SetPlayerCharacter _asbp_player_character)
  (Variables|/Game/Blueprints/BPC_ItemGenerator.BPC_ItemGenerator_C|SetConstructionAsset (Variables|Default|GetBPS_ItemGenerator) self))

(event EventActorBeginOverlap
  (params (OtherActor :type Actor%20Object%20Reference)))

(event EventTick
  (params (DeltaSeconds :type Float%20%28single-precision%29)))

(event Input|ActionEvents|InputActionAction
  (params (Key :type Key%20Structure :default "AnyKey"))
  (:Pressed
    (if (Variables|/Game/Blueprints/BPC_ItemGenerator.BPC_ItemGenerator_C|GetEnabled (Variables|Default|GetBPS_ItemGenerator))
      (if (Variables|/Game/Blueprints/BPC_ItemGenerator.BPC_ItemGenerator_C|GetItemsGenerated (Variables|Default|GetBPS_ItemGenerator))
        (for _array_element (Variables|/Game/Blueprints/BPC_ItemGenerator.BPC_ItemGenerator_C|GetGeneratedItems (Variables|Default|GetBPS_ItemGenerator))
          (Default|AddItemtoInventory (Variables|Default|GetPlayerCharacter) _array_element))
        (Default|ResetTimer (Variables|Default|GetBPS_ItemGenerator))))))

(fn ConstructionScript)

(fn UpdateTextRender
  (params (VisibilityState :type Boolean))
  (Rendering|SetVisibility (Variables|Default|GetTextRender) VisibilityState false))